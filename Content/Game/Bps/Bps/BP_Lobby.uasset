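; BP_Lobby is a lobby actor that displays the player's selectable character with a name text.
; BeginPlay opens the WB_changeChar widget with a reference to itself and caches MY_GI.
; UpdateChar maps the game instance's Chars selection to one of twelve Noir or SurvGirl skeletal meshes.
; MC_ events set the name and play one-shot animations on the character; MC_setCharMesh is an empty stub.
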(event `self.ReceiveBeginPlay`
  (bind _returnvalue (`|CreateWidget` "/Game/Game/Bps/Bps/WB_changeChar.WB_changeChar_C"))
  (bind _output_get (set `self.Widget` _returnvalue))
  (set `/Game/Game/Bps/Bps/WB_changeChar.bp` self _output_get)
  (`UserWidget.AddToViewport` _output_get 0)
  (bind _asmy_gi (cast `/Game/Game/Bps/MY_GI` (`GameplayStatics.GetGameInstance`)))
  (set `self.As MY GI` _asmy_gi))

(event `MC_setPlayerName`
  (params (PlayerName :type Text))
  (`self.SetPlayerName` PlayerName))

(event `MC_setCharMesh`
  (params (NewMesh :type "SkeletalMesh Object Reference")))

(event `MC_PLAYMeshAnims`
  (params (NewAnimToPlay :type "AnimationAsset Object Reference"))
  (`SkeletalMeshComponent.PlayAnimation` (`self.Char`) NewAnimToPlay false))

(event `/Game/Game/Bps/Bps/ChangeChar.UpdateChar`
  (switch `/Game/Game/Bps/Bps/E_Chars` (`/Game/Game/Bps/MY_GI.Chars` (`self.As MY GI`))
    (:`NewEnumerator0`
      (`SkeletalMeshComponent.SetSkeletalMeshAsset` (`self.Char`) "/Game/Noir/Meshes/SK_Noir_SetA2.SK_Noir_SetA2"))
    (:`NewEnumerator1`
      (`SkeletalMeshComponent.SetSkeletalMeshAsset` (`self.Char`) "/Game/Noir/Meshes/SK_Noir_SetB2.SK_Noir_SetB2"))
    (:`NewEnumerator2`
      (`SkeletalMeshComponent.SetSkeletalMeshAsset` (`self.Char`) "/Game/Noir/Meshes/SK_Noir_SetC.SK_Noir_SetC"))
    (:`NewEnumerator3`
      (`SkeletalMeshComponent.SetSkeletalMeshAsset` (`self.Char`) "/Game/SurvivalGirl/Mesh/Combinations/SK_SurvGirl_Combination01.SK_SurvGirl_Combination01"))
    (:`NewEnumerator4`
      (`SkeletalMeshComponent.SetSkeletalMeshAsset` (`self.Char`) "/Game/SurvivalGirl/Mesh/Combinations/SK_SurvGirl_Combination02.SK_SurvGirl_Combination02"))
    (:`NewEnumerator5`
      (`SkeletalMeshComponent.SetSkeletalMeshAsset` (`self.Char`) "/Game/SurvivalGirl/Mesh/Combinations/SK_SurvGirl_Combination03.SK_SurvGirl_Combination03"))
    (:`NewEnumerator6`
      (`SkeletalMeshComponent.SetSkeletalMeshAsset` (`self.Char`) "/Game/SurvivalGirl/Mesh/Combinations/SK_SurvGirl_Combination04.SK_SurvGirl_Combination04"))
    (:`NewEnumerator7`
      (`SkeletalMeshComponent.SetSkeletalMeshAsset` (`self.Char`) "/Game/SurvivalGirl/Mesh/Combinations/SK_SurvGirl_Combination05.SK_SurvGirl_Combination05"))
    (:`NewEnumerator8`
      (`SkeletalMeshComponent.SetSkeletalMeshAsset` (`self.Char`) "/Game/SurvivalGirl/Mesh/Combinations/SK_SurvGirl_Combination06.SK_SurvGirl_Combination06"))
    (:`NewEnumerator9`
      (`SkeletalMeshComponent.SetSkeletalMeshAsset` (`self.Char`) "/Game/SurvivalGirl/Mesh/Combinations/SK_SurvGirl_Combination07.SK_SurvGirl_Combination07"))
    (:`NewEnumerator10`
      (`SkeletalMeshComponent.SetSkeletalMeshAsset` (`self.Char`) "/Game/SurvivalGirl/Mesh/Combinations/SK_SurvGirl_Combination08.SK_SurvGirl_Combination08"))
    (:`NewEnumerator11`
      (`SkeletalMeshComponent.SetSkeletalMeshAsset` (`self.Char`) "/Game/SurvivalGirl/Mesh/Combinations/SK_SurvGirl_Combination09.SK_SurvGirl_Combination09"))))

(fn `SetPlayerName`
  (params (PlayerName :type Text))
  (`TextRenderComponent.K2_SetText` (`self.PlayerName`) PlayerName)
  (return))

(fn `UserConstructionScript`)