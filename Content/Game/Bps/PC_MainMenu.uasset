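; Main menu player controller that manages the menu screens for main menu, server creation and server browser.
; On BeginPlay it shows the main menu through ShowHideWidget, which acts only on the local player controller and routes to ShowWidget or HideWidget by a widget selector.
; Each widget is created lazily on first show, cached, then added to or removed from the viewport.
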(event `self.ReceiveBeginPlay`
  (`self.ShowHideWidget` "NewEnumerator0" true))

(event `ShowHideWidget`
  (params (Widget :type "/Game/Game/Enums/MainMenuWidgets Enum" :default "NewEnumerator0") (Show :type Boolean))
  (if (`self.IsLocalPlayerController`)
    (if Show
      (`self.ShowWidget` Widget)
      (else
        (`self.HideWidget` Widget)))))

(fn `GetPlayerControllerRef`
  (returns (PlayerController :type "/Game/Game/Bps/PC_MainMenu Object Reference"))
  (return self))

(fn `HideWidget`
  (params (Widgets :type "/Game/Game/Enums/MainMenuWidgets Enum" :default "NewEnumerator0"))
  (switch `/Game/Game/Enums/MainMenuWidgets` Widgets
    (:`NewEnumerator0`
      (bind _mainmenu (`self.MainMenu`)
        (:`then`
          (`Widget.RemoveFromParent` _mainmenu))
        (:`else`)))
    (:`NewEnumerator1`
      (bind _createserver (`self.CreateServer`)
        (:`then`
          (`Widget.RemoveFromParent` _createserver))
        (:`else`)))
    (:`NewEnumerator2`
      (bind _serverbrowser (`self.ServerBrowser`)
        (:`then`
          (`Widget.RemoveFromParent` _serverbrowser))
        (:`else`)))))

(fn `ShowWidget`
  (params (Widgets :type "/Game/Game/Enums/MainMenuWidgets Enum" :default "NewEnumerator0"))
  (switch `/Game/Game/Enums/MainMenuWidgets` Widgets
    (:`NewEnumerator0`
      (`self.MainMenu`
        (:`then`
          _)
        (:`else`
          (bind _returnvalue (`|CreateWidget` "/Game/Game/UI/WB_MainMenu.WB_MainMenu_C"))
          (bind _output_get (set `self.MainMenu` _returnvalue))))
      (`UserWidget.AddToViewport` _output_get 0))
    (:`NewEnumerator1`
      (`self.CreateServer`
        (:`then`
          _)
        (:`else`
          (bind _returnvalue_2 (`|CreateWidget` "/Game/Game/UI/WB_createServer.WB_createServer_C"))
          (bind _output_get_2 (set `self.CreateServer` _returnvalue_2))))
      (`UserWidget.AddToViewport` _output_get_2 0))
    (:`NewEnumerator2`
      (`self.ServerBrowser`
        (:`then`
          _)
        (:`else`
          (bind _returnvalue_3 (`|CreateWidget` "/Game/Game/UI/WB_serverBrowser.WB_serverBrowser_C"))
          (bind _output_get_3 (set `self.ServerBrowser` _returnvalue_3))))
      (`UserWidget.AddToViewport` _output_get_3 0))))

(fn `UserConstructionScript`)